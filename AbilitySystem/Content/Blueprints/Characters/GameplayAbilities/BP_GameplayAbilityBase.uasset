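; Base Gameplay Ability Blueprint providing shared helpers for specific abilities, mainly to show cooldowns in the player's UI.
; GetPlayerCharacerAndController casts the owning actor to BP_CharacterBase and its controller to BP_PlayerController.
; DoUICoolDown, called by specific abilities after Commit Ability, starts the cooldown on PrimaryUI slots whose ability class matches the one from GetAbilityInfo.
; The activate and end events are unimplemented here.
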(fn `DoUICoolDown`
  (bind (_characterbase _playercontroller) (`self.GetPlayerCharacerAndController`))
  (`/Engine/EditorBlueprintResources/StandardMacros.IsValid` _playercontroller
    (:`Is Valid`
      (for _array_element (`/Game/UI/WBP_PrimaryUI.Slots` (`/Game/Blueprints/BP_PlayerController.PrimaryUI` _playercontroller))
        (bind _returnvalue (`self.GetAbilityInfo`))
        (bind (_abilityinfo_cooldownduration _abilityinfo_cost _abilityinfo_costtype _abilityinfo_uimat _abilityinfo_abilityclass) (break `GameplayAbilityInfo` (`/Game/UI/WBP_Ability_Slot.AbilityInfo` _array_element)))
        (if (== _abilityinfo_abilityclass (`.AbilityClass` (break `GameplayAbilityInfo` _returnvalue)))
          (`/Game/UI/WBP_Ability_Slot.StartCoolDown` _array_element) ; Get the corresponding slot to do the cooldown
        )))))

(fn `GetPlayerCharacerAndController`
  (returns (CharacterBase :type "/Game/Blueprints/Characters/BP_CharacterBase Object Reference") (PlayerController :type "/Game/Blueprints/BP_PlayerController Object Reference"))
  (bind _asbp_character_base (cast `/Game/Blueprints/Characters/BP_CharacterBase` (`self.GetOwningActorFromActorInfo`)))
  (bind _asbp_player_controller (cast `/Game/Blueprints/BP_PlayerController` (`Pawn.GetController` _asbp_character_base))
    (:`then`
      _)
    (:`CastFailed`
      _))
  (return _asbp_character_base _asbp_player_controller))