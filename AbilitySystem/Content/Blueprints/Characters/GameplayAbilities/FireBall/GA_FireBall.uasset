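; Gameplay ability that casts a fireball from the player character after a melee combo montage.
; On activation it commits, triggers the UI cooldown and plays the Shinbi montage.
; Completion or blend-out spawns BP_FireBall at the character's transform, passing the character as instigator and a GE_Dash_Damage effect spec, then ends the ability.
; Interruption or cancellation ends it without spawning.
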(event `self.K2_ActivateAbility`
  (`self.K2_CommitAbility`)
  (`self.DoUICoolDown`)
  (`AbilityTask_PlayMontageAndWait.CreatePlayMontageAndWaitProxy` "None" "/Game/Blueprints/Characters/Animation/AM_Shinbi_Melee_Combo_03.AM_Shinbi_Melee_Combo_03"
    (:`OnCompleted`
      (bind _characterbase (`self.GetPlayerCharacerAndController` :!label _label))
      (`|SpawnActorFromClass` "/Game/Blueprints/Characters/GameplayAbilities/FireBall/BP_FireBall.BP_FireBall_C" (`Actor.GetTransform` _characterbase) "AlwaysSpawn" "OverrideRootScale" null (`self.MakeOutgoingGameplayEffectSpec` "/Game/Blueprints/Characters/GameplayAbilities/Dash/GE_Dash_Damage.GE_Dash_Damage_C") _characterbase)
      (`self.K2_EndAbility`))
    (:`OnBlendOut`
      (goto _label))
    (:`OnInterrupted`
      (`self.K2_EndAbility` :!label _label_2))
    (:`OnCancelled`
      (goto _label_2))))