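; GA_Lazer is a Gameplay Ability that casts a laser from the player character and damages targets.
; On activation it commits, starts the UI cooldown and casting montage, then after a short delay spawns BP_Lazer on the mesh's "Lazer" socket and enables camera-controlled rotation.
; It applies GE_Lazer_Damage to target data received through the Skill.lazer.dealDamage gameplay event.
; The graph never calls EndAbility.
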(event `self.K2_ActivateAbility`
  (`self.K2_CommitAbility`)
  (`self.DoUICoolDown`)
  (`AbilityTask_PlayMontageAndWait.CreatePlayMontageAndWaitProxy` "None" "/Game/Blueprints/Characters/Animation/AM_Lazer_Casting.AM_Lazer_Casting"
    (:`then`
      (`KismetSystemLibrary.Delay` 0.3)
      (bind _characterbase (`self.GetPlayerCharacerAndController`))
      (bind (_asynctaskproxy _spawnedactor) (`AbilityTask_SpawnActor.SpawnActor` (struct) "/Game/Blueprints/Characters/GameplayAbilities/Lazer/BP_Lazer.BP_Lazer_C" _characterbase)
        (:`then`
          (bind _output_get (set `self.LazerActor` _spawnedactor))
          (`Actor.K2_AttachToComponent` _output_get (`Character.Mesh` _characterbase) "Lazer" "SnapToTarget" "SnapToTarget" "KeepRelative" true)
          (`/Game/Blueprints/Characters/BP_CharacterBase.MakeCameraControlRotation` _characterbase true)
          (bind (_asynctaskproxy_2 _payload) (`AbilityTask_WaitGameplayEvent.WaitGameplayEvent` (struct :`TagName` "skill.lazer.dealDamage") null)
            (:`EventReceived`
              (`self.BP_ApplyGameplayEffectToTarget` (`.TargetData` (break `GameplayEventData` _payload)) "/Game/Blueprints/Characters/GameplayAbilities/Lazer/GE_Lazer_Damage.GE_Lazer_Damage_C"))))))))